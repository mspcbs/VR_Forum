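; BP_ForumGameMode is a game mode Blueprint that numbers and names the VR pawns in the level.
; On BeginPlay it waits through a short delay, then gathers every BP_VRPawn actor.
; For each one it sets the player ID to the array index, builds a "Player" plus index name, and increments a player count.
; Pawns that appear after this single pass are not registered here.
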(event EventBeginPlay
  (Utilities|FlowControl|Delay 3.0)
  (bind _outactors (Actor|GetAllActorsOfClass "/Game/Blueprints/BP_VR-Pawn.BP_VR-Pawn_C"))
  (for (_array_element _array_index) _outactors
    (bind _asbp_vr_pawn (Utilities|Casting|CastToBP_VR-Pawn _array_element))
    (Default|SetPlayerID _asbp_vr_pawn _array_index)
    (Default|SetPlayerName _asbp_vr_pawn (Utilities|Text|ToText(String) (Utilities|String|Append (Utilities|String|MakeLiteralString "Player ") (Utilities|String|ToString(Integer) _array_index))))
    (Math|Integer|IncrementInt (Variables|Default|Geti_NumberOfPlayers))))

(fn ConstructionScript)