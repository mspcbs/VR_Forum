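; BP_MenuPawn is a VR menu pawn that lets the player operate widget UI with the right motion controller trigger.
; BeginPlay sets a floor tracking origin, and the trigger presses and releases the WidgetInteraction pointer as a left mouse click.
; Each Tick moves InteractionSphere to just before the pointer's last hit point.
; Helpers to align the pointer to the right controller and give both hands a shared dynamic material are defined but not called here.
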(event Custom|WidgetInteractionLocation
  ;[1 1 1] LOCAL UI
  ;;[1 1 1] Set WidgetInteraction to HandLocation
  (CallFunction|UpdateInteractionHitLocation))

(event EventBeginPlay
  (Utilities|FlowControl|Sequence
    (:then_0
      ;[0 0 0] Setup Player Height
      (Class|HeadMountedDisplayFunctionLibrary|SetTrackingOrigin "Floor") ; Windows (Oculus / Vive)
    )))

(event EventTick
  (params (DeltaSeconds :type Float%20%28single-precision%29))
  (CallFunction|WidgetInteractionLocation))

(event Input|ActionEvents|InputActionTrigger_Right
  (params (Key :type Key%20Structure))
  (bind _widgetinteraction (Variables|Default|GetWidgetInteraction))
  ;[1 1 1] LOCAL UI
  ;;[1 1 1] Only Allow MotionController to Interact
  (:Pressed
    (Class|WidgetInteractionComponent|PressPointerKey _widgetinteraction "LeftMouseButton"))
  (:Released
    (Class|WidgetInteractionComponent|ReleasePointerKey _widgetinteraction "LeftMouseButton")))

(fn ConstructionScript)

(fn InteractionLocation
  (params (MotionController :type %20Object%20Reference) (WidgetInteraction :type Widget%20Interaction%20Component%20Object%20Reference))
  (bind _motioncontroller_r (Variables|Default|GetMotionController_R))
  (Transformation|SetWorldLocationAndRotation WidgetInteraction (Transformation|GetWorldLocation _motioncontroller_r) (Transformation|GetWorldRotation _motioncontroller_r) false false))

(fn UpdateInteractionHitLocation
  (bind _widgetinteraction (Variables|Default|GetWidgetInteraction))
  (bind _output_get (Variables|UI|Setv_InteractionHitLocation (+ (Transformation|GetWorldLocation _widgetinteraction) (* (Math|Vector|GetForwardVector _widgetinteraction) (- (.Distance (Collision|BreakHitResult (Class|WidgetInteractionComponent|GetLastHitResult _widgetinteraction))) 1.0)))))
  (Transformation|SetWorldLocation (Variables|Default|GetInteractionSphere) _output_get false false))

(fn CreateDynMatInst
  (bind _handmesh_left (Variables|Default|GetHandMesh_Left))
  (bind _returnvalue (Rendering|Material|CreateDynamicMaterialInstance _handmesh_left 0 "/Game/Assets/Materials/Avatar/Avatar_Master.Avatar_Master" "PawnColor" :!class /Script/Engine.PrimitiveComponent))
  (Rendering|Material|SetMaterial _handmesh_left 0 _returnvalue)
  (return))