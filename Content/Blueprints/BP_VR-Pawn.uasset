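; Networked VR player pawn with thumbstick movement and turning, an avatar head, hands and name tag, and per-player colour via a replicated player ID.
; The locally controlled pawn sends head and controller transforms by RPC each Tick to drive the avatar, and hides its own head and tag.
; Stick input runs locally and through server or multicast events.
; It spawns a toggleable floating UI, clicked with a right-trigger widget pointer.
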(event Custom|WidgetInteractionLocation
  ;[1 1 1] LOCAL UI
  ;;[1 1 1] Set WidgetInteraction to HandLocation
  (CallFunction|UpdateInteractionHitLocation))

(event Custom|MC_Movement%20Y%20Left
  (params (AxisValue :type Float%20%28single-precision%29))
  ;[1 1 1] Thumbstick Locomotion
  (CallFunction|MovementYLeft AxisValue))

(event Custom|ROS_UpdateHead
  (params (HeadRot :type Rotator) (HeadPos :type Vector))
  ;[0.2188 0 0] Component Network Update
  ;;[1 1 1] Head
  ;;;[1 0 0] ROS
  (Variables|Networking|Setr_HeadRot HeadRot)
  (Variables|Networking|Setv_HeadPos HeadPos))

(event Custom|UpdateHand
  (params (HandPos :type Vector) (HandRot :type Rotator) (Hand :type Scene%20Component%20Object%20Reference))
  ;[0.2188 0 0] Component Network Update
  ;;[1 1 1] Hands
  ;;;[1 0 0] ROS
  (Transformation|SetWorldLocation Hand HandPos false false)
  (Transformation|SetWorldRotation Hand HandRot false false))

(event Custom|UpdateHandsPos
  (bind _motioncontroller_l (Variables|Default|GetMotionController_L))
  (bind _motioncontroller_r (Variables|Default|GetMotionController_R))
  ;[0.2188 0 0] Component Network Update
  ;;[1 1 1] Hands
  (if (Pawn|IsLocallyControlled)
    ;;;[1 1 1] Left Controller
    (Variables|Networking|Setv_ControllerL_Pos (Transformation|GetWorldLocation _motioncontroller_l))
    (Variables|Networking|Setr_ControllerL_Rot (Transformation|GetWorldRotation _motioncontroller_l))
    ;;;[1 1 1] Left Controller
    (Variables|Networking|Setv_ControllerR_Pos (Transformation|GetWorldLocation _motioncontroller_r))
    (Variables|Networking|Setr_ControllerR_Rot (Transformation|GetWorldRotation _motioncontroller_r))
    ;;;[1 0 0] RPC
    (CallFunction|ROSUpdateHand (Variables|Networking|Getv_ControllerR_Pos) (Variables|Networking|Getr_ControllerR_Rot) (Variables|Networking|Getv_ControllerL_Pos) (Variables|Networking|Getr_ControllerL_Rot)))
  (CallFunction|UpdateHand (Variables|Networking|Getv_ControllerR_Pos) (Variables|Networking|Getr_ControllerR_Rot) (Variables|Default|GetHand_Right_Container))
  (CallFunction|UpdateHand (Variables|Networking|Getv_ControllerL_Pos) (Variables|Networking|Getr_ControllerL_Rot) (Variables|Default|GetHand_Left_Container)))

(event Custom|ROS_UpdateHand
  (params (ControllerR_Pos :type Vector) (ControllerR_Rot :type Rotator) (ControllerL_Pos :type Vector) (ControllerL_Rot :type Rotator))
  ;[0.2188 0 0] Component Network Update
  ;;[1 1 1] Hands
  ;;;[1 0 0] ROS
  (Variables|Networking|Setv_ControllerR_Pos ControllerR_Pos)
  (Variables|Networking|Setr_ControllerR_Rot ControllerR_Rot)
  (Variables|Networking|Setv_ControllerL_Pos ControllerL_Pos)
  (Variables|Networking|Setr_ControllerL_Rot ControllerL_Rot))

(event Custom|MC_Rotation%20X%20Right
  (params (Rotation%20Angle :type Float%20%28single-precision%29))
  ;[1 1 1] Thumbstick Locomotion
  (CallFunction|RotationXRight Rotation%20Angle))

(event Custom|UpdatePlayerNamePos
  (bind _v_headpos (Variables|Networking|Getv_HeadPos))
  ;[1 1 1] LOCAL UI
  ;;[0.8298 1 0.3785] Player Name
  (Transformation|SetWorldLocation (Variables|Default|GetNameTag) (Math|Vector|MakeVector (.x _v_headpos) (.y _v_headpos) (+ (.z _v_headpos) 45.0)) false false))

(event Custom|MC_Movement%20X%20Left
  (params (Axis%20Value :type Float%20%28single-precision%29))
  ;[1 1 1] Thumbstick Locomotion
  (CallFunction|MovementXLeft Axis%20Value))

(event Custom|UpdateHeadPos
  (bind _camera (Variables|Default|GetCamera))
  ;[0.2188 0 0] Component Network Update
  ;;[1 1 1] Head
  (if (Pawn|IsLocallyControlled)
    (Variables|Networking|Setv_HeadPos (Transformation|GetWorldLocation _camera))
    (Variables|Networking|Setr_HeadRot (Transformation|GetWorldRotation _camera))
    (CallFunction|ROSUpdateHead (Variables|Networking|Getr_HeadRot) (Variables|Networking|Getv_HeadPos)))
  (Transformation|SetWorldLocation (Variables|Default|GetHead) (Variables|Networking|Getv_HeadPos) false false)
  (Transformation|SetWorldRotation (Variables|Default|GetHead) (Variables|Networking|Getr_HeadRot) false false))

(event Custom|ROS_Movement%20X%20Left
  (params (AxisValue :type Float%20%28single-precision%29))
  ;[1 1 1] Thumbstick Locomotion
  (CallFunction|MovementXLeft (stale Custom|MC_Movement%20X%20Left Axis%20Value)))

(event Custom|ROS_Movement%20Y%20Left
  (params (AxisValue :type Float%20%28single-precision%29))
  ;[1 1 1] Thumbstick Locomotion
  (CallFunction|MovementYLeft (stale Custom|MC_Movement%20Y%20Left AxisValue)))

(event Custom|ROS_Rotation%20X%20Right
  (params (AxisValue :type Float%20%28single-precision%29))
  ;[1 1 1] Thumbstick Locomotion
  (CallFunction|RotationXRight (stale Custom|MC_Rotation%20X%20Right Rotation%20Angle)))

(event EventBeginPlay
  (bind _self self)
  (Utilities|FlowControl|Sequence
    (:then_0
      ;[0 0 0] Setup Player Height
      (Class|HeadMountedDisplayFunctionLibrary|SetTrackingOrigin "Floor") ; Windows (Oculus / Vive)
    )
    (:then_1
      ;[1 1 1] Spawn and Attach Floating UI
      (bind _returnvalue (Game|SpawnActorfromClass "/Game/UI/FloatingUI/BP_FloatingUI.BP_FloatingUI_C" (Transformation|GetWorldTransform (Variables|Default|GetVROrigin)) "AlwaysSpawn" _self _self))
      (Variables|/Game/UI/FloatingUI/BP_FloatingUI.BP_FloatingUI_C|SetBP_VR-Pawn _returnvalue self)
      (Variables|UI|SetBP_FloatingUI _returnvalue)
      (Variables|UI|Setb_HasFloatingUI true)
      (Default|ToggleUI _returnvalue))
    (:then_2
      ;[1 1 1] Hide HMD Model + NameTag on Owned Pawn
      (if (Pawn|IsLocallyControlled)
        (Rendering|SetVisibility (Variables|Default|GetHead) false false)
        (Rendering|Material|SetMaterial (Variables|Default|GetHandMesh_Left) 0 "/Game/Assets/Materials/Avatar/Avatar_Inst.Avatar_Inst")))))

(event EventTick
  (params (DeltaSeconds :type Float%20%28single-precision%29))
  (Utilities|FlowControl|Sequence
    (:then_0
      ;[1 0 0] Networking
      (CallFunction|UpdateHeadPos)
      (CallFunction|UpdateHandsPos))
    (:then_1
      (CallFunction|WidgetInteractionLocation))
    (:then_2
      (CallFunction|UpdatePlayerNamePos))))

(event Input|ActionEvents|InputActionUI_Left
  (params (Key :type Key%20Structure :default "None"))
  (bind _bp_floatingui (Variables|UI|GetBP_FloatingUI))
  ;[1 1 1] LOCAL UI
  ;;[1 1 1] Floating Menu
  (:Pressed
    (Utilities|IsValid _bp_floatingui
      (:Is%20Valid
        (Default|ToggleUI _bp_floatingui)))))

(event Input|ActionEvents|InputActionUI_Right
  (params (Key :type Key%20Structure :default "None"))
  (bind _bp_floatingui (Variables|UI|GetBP_FloatingUI))
  ;[1 1 1] LOCAL UI
  ;;[1 1 1] Floating Menu
  (:Pressed
    (Utilities|IsValid _bp_floatingui
      (:Is%20Valid
        (Default|ToggleUI _bp_floatingui)))))

(event Input|ActionEvents|InputActionTrigger_Right
  (params (Key :type Key%20Structure :default "None"))
  (bind _widgetinteraction (Variables|Default|GetWidgetInteraction))
  ;[1 1 1] LOCAL UI
  ;;[1 1 1] Only Allow MotionController to Interact
  (:Pressed
    (Class|WidgetInteractionComponent|PressPointerKey _widgetinteraction "LeftMouseButton"))
  (:Released
    (Class|WidgetInteractionComponent|ReleasePointerKey _widgetinteraction "LeftMouseButton")))

(event Input|AxisEvents|InputAxisMotionControllerThumbLeft_X
  (params (AxisValue :type Float%20%28single-precision%29))
  ;[1 1 1] Thumbstick Locomotion
  (Networking|SwitchHasAuthority
    (:Authority
      (CallFunction|MCMovementXLeft AxisValue))
    (:Remote
      (CallFunction|ROSMovementXLeft AxisValue)))
  (CallFunction|MovementXLeft AxisValue))

(event Input|AxisEvents|InputAxisMotionControllerThumbLeft_Y
  (params (AxisValue :type Float%20%28single-precision%29))
  ;[1 1 1] Thumbstick Locomotion
  (Networking|SwitchHasAuthority
    (:Authority
      (CallFunction|MCMovementYLeft AxisValue))
    (:Remote
      (CallFunction|ROSMovementYLeft AxisValue)))
  (CallFunction|MovementYLeft AxisValue))

(event Input|AxisEvents|InputAxisMotionControllerThumbRight_X
  (params (AxisValue :type Float%20%28single-precision%29))
  ;[1 1 1] Thumbstick Locomotion
  (Networking|SwitchHasAuthority
    (:Authority
      (CallFunction|MCRotationXRight AxisValue))
    (:Remote
      (CallFunction|ROSRotationXRight AxisValue)))
  (CallFunction|RotationXRight AxisValue))

(fn ConstructionScript)

(fn GetRotationfromInput
  (params (UpAxis :type Float%20%28single-precision%29) (RightAxis :type Float%20%28single-precision%29) (Controller :type %20Object%20Reference)))

(fn InteractionLocation
  (params (MotionController :type %20Object%20Reference) (WidgetInteraction :type Widget%20Interaction%20Component%20Object%20Reference))
  (bind _motioncontroller_r (Variables|Default|GetMotionController_R))
  (Transformation|SetWorldLocationAndRotation WidgetInteraction (Transformation|GetWorldLocation _motioncontroller_r) (Transformation|GetWorldRotation _motioncontroller_r) false false))

(fn UpdateInteractionHitLocation
  (bind _widgetinteraction (Variables|Default|GetWidgetInteraction))
  (bind _interactionsphere (Variables|Default|GetInteractionSphere))
  (bind _returnvalue (Class|WidgetInteractionComponent|GetLastHitResult _widgetinteraction))
  (bind _distance (Collision|BreakHitResult _returnvalue))
  (bind _output_get (Variables|UI|Setv_InteractionHitLocation (+ (Transformation|GetWorldLocation _widgetinteraction) (* (Math|Vector|GetForwardVector _widgetinteraction) (- _distance 1.0)))))
  (Transformation|SetWorldLocation (Variables|Default|GetInteractionSphere) _output_get false false)
  (if (<= _distance 5e+01)
    (Rendering|SetVisibility _interactionsphere false false)
    (else
      (Rendering|SetVisibility _interactionsphere true false))))

(fn MovementXLeft
  (params (InputPin :type Float%20%28single-precision%29))
  (bind _vrorigin (Variables|Default|GetVROrigin))
  (bind _returnvalue (Math|Vector|GetRightVector _vrorigin))
  (if (not (== InputPin 0.0))
    (Pawn|Input|AddMovementInput (Math|Vector|MakeVector (.x _returnvalue) (.y _returnvalue) 0.0) (* InputPin (Variables|Locomotion|Getf_MovementSpeed)) false)))

(fn MovementYLeft
  (params (InputPin :type Float%20%28single-precision%29))
  (bind _vrorigin (Variables|Default|GetVROrigin))
  (bind _returnvalue (Math|Vector|GetForwardVector _vrorigin))
  (if (not (== InputPin 0.0))
    (Pawn|Input|AddMovementInput (Math|Vector|MakeVector (.x _returnvalue) (.y _returnvalue) 0.0) (* InputPin (Variables|Locomotion|Getf_MovementSpeed)) false)))

(fn RotationXRight
  (params (Rotation%20Angle :type Float%20%28single-precision%29))
  (bind _returnvalue (Transformation|GetActorTransform))
  (Variables|Locomotion|Setf_Rotation%20Angle Rotation%20Angle)
  (Transformation|SetActorTransform (Math|Transform|MakeTransform (.location _returnvalue) (Math|Rotator|MakeRotator 0.0 0.0 (+ (.yaw (Transformation|GetActorRotation)) (* (Variables|Locomotion|Getf_Rotation%20Angle) (Variables|Locomotion|Getf_RotationSpeed)))) (.scale _returnvalue))))

(fn CreateDynMatInst
  (bind _returnvalue (Rendering|Material|CreateDynamicMaterialInstance (Variables|Default|GetHead) 0 "/Game/Assets/Materials/Avatar/Avatar_Master.Avatar_Master" "PawnColor" :!class /Script/Engine.PrimitiveComponent))
  (bind _output_get (Variables|Networking|Setm_PlayerColor_MatInst _returnvalue))
  (Rendering|Material|SetMaterial (Variables|Default|GetHandMesh_Left) 0 _output_get)
  (return))

(fn SetPlayerID
  (params (PlayerID :type Integer))
  (Variables|Networking|Seti_PlayerID PlayerID))

(fn OnRepPlayerID
  (bind _m_playercolor_matinst (Variables|Networking|Getm_PlayerColor_MatInst))
  (Utilities|IsValid _m_playercolor_matinst
    (:Is%20Valid
      _)
    (:Is%20Not%20Valid
      (CallFunction|CreateDynMatInst)))
  (switch int (Variables|Networking|Geti_PlayerID)
    (:Default
      (Rendering|Material|SetVectorParameterValue _m_playercolor_matinst "Color" "(R=0.567708,G=0.041225,B=0.000000,A=1.000000)" :!class /Script/Engine.MaterialInstanceDynamic))
    (:0
      (Rendering|Material|SetVectorParameterValue _m_playercolor_matinst "Color" "(R=0.302083,G=0.292883,B=0.017307,A=1.000000)" :!class /Script/Engine.MaterialInstanceDynamic))
    (:1
      (Rendering|Material|SetVectorParameterValue _m_playercolor_matinst "Color" "(R=0.073079,G=0.333333,B=0.138142,A=1.000000)" :!class /Script/Engine.MaterialInstanceDynamic))
    (:2
      (Rendering|Material|SetVectorParameterValue _m_playercolor_matinst "Color" "(R=0.020508,G=0.179533,B=0.187500,A=1.000000)" :!class /Script/Engine.MaterialInstanceDynamic))
    (:3
      (Rendering|Material|SetVectorParameterValue _m_playercolor_matinst "Color" "(R=0.239192,G=0.104708,B=0.359375,A=1.000000)" :!class /Script/Engine.MaterialInstanceDynamic))))

(fn SetPlayerName
  (params (PlayerName :type Text))
  (Variables|Networking|Setnm_PlayerName PlayerName))